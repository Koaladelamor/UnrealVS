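; Enemy character that attacks a random point around the BP_Sanctum, switching to chase the player when PawnSensing spots them.
; AIMoveTo retries on failure and triggers a swipe on arrival; separate CheckAttack and EndAttack events sphere-trace damage and resume movement.
; Externally called Headshot and Bodyshot events subtract health, with body hits staggering and death destroying the actor after a delay.
; Tick zeroes speed on moving corpses as a hotfix.
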(event `EndAttack`
  (`KismetSystemLibrary.Delay` 1.4)
  (set `CharacterMovementComponent.MaxWalkSpeed` 300.0 (`self.CharacterMovement`))
  (`SkeletalMeshComponent.SetAnimationMode` (`self.Mesh`) "AnimationBlueprint")
  (if (`self.ChasingPlayer`)
    (`self.Chase Player`)
    (else
      (`self.MoveToSanctuary`))))

(event `CheckAttack`
  (bind _attackposition (`self.AttackPosition`))
  (bind _returnvalue (`SceneComponent.K2_GetComponentLocation` _attackposition))
  (bind (_outhit _returnvalue_2) (`KismetSystemLibrary.SphereTraceSingle` _returnvalue (+ _returnvalue (* (`KismetMathLibrary.GetForwardVector` (`SceneComponent.K2_GetComponentRotation` _attackposition)) 40.0)) 25.0 "TraceTypeQuery1"))
  (if _returnvalue_2
    (bind (_bblockinghit _binitialoverlap _time _distance _location _impactpoint _normal _impactnormal _physmat _hitactor _hitcomponent) (`GameplayStatics.BreakHitResult` _outhit))
    (bind _asbp_sanctum (cast `/Game/FirstPerson/Sanctuary/BP_Sanctum` _hitactor)
      (:`then`
        (`/Game/FirstPerson/Sanctuary/BP_Sanctum.ReceiveDamage` _asbp_sanctum))
      (:`CastFailed`
        (bind _asbp_first_person_character (cast `/Game/FirstPerson/Blueprints/BP_FirstPersonCharacter` _hitactor)
          (:`then`
            (`/Game/FirstPerson/Blueprints/BP_FirstPersonCharacter.ReceiveDamage` _asbp_first_person_character 10.0))
          (:`CastFailed`
            (`KismetSystemLibrary.PrintString` (`KismetSystemLibrary.GetDisplayName` _hitcomponent))))))
    (else
      (`KismetSystemLibrary.PrintString` "no hit"))))

(event `Attack`
  (set `CharacterMovementComponent.MaxWalkSpeed` 0.0 (`self.CharacterMovement`))
  (`SkeletalMeshComponent.PlayAnimation` (`self.Mesh`) "/Game/Enemy/Animations/Mutant_Swiping.Mutant_Swiping" false))

(event `MoveToSanctuary`
  (bind (_returnvalue_roll _returnvalue_pitch) (`KismetMathLibrary.BreakRotator` (`self.K2_GetActorRotation`)))
  (bind _sanctuaryref (`self.SanctuaryRef`))
  (bind (_returnvalue_roll_2 _returnvalue_pitch_2 _returnvalue_yaw) (`KismetMathLibrary.BreakRotator` (`KismetMathLibrary.FindLookAtRotation` (`self.K2_GetActorLocation`) (`self.K2_GetActorLocation` _sanctuaryref))))
  (if (not (`self.Dead`))
    (switch `int` (`KismetMathLibrary.RandomInteger` 3)
      (:`0`
        (`|AIMoveTo` self (`SceneComponent.K2_GetComponentLocation` (`/Game/FirstPerson/Sanctuary/BP_Sanctum.AttackPoint1` _sanctuaryref)) null
          (:`OnSuccess`
            (if (not (`self.Dead`)) :!label _label
              (`self.K2_SetActorRotation` (`KismetMathLibrary.MakeRotator` _returnvalue_roll _returnvalue_pitch _returnvalue_yaw))
              (`self.Attack`)))
          (:`OnFail`
            (`KismetSystemLibrary.Delay` 0.2 :!label _label_2)
            (if (`self.ChasingPlayer`)
              (`self.Chase Player`)
              (else
                (`self.MoveToSanctuary`))))))
      (:`1`
        (`|AIMoveTo` self (`SceneComponent.K2_GetComponentLocation` (`/Game/FirstPerson/Sanctuary/BP_Sanctum.AttackPoint2` _sanctuaryref)) null
          (:`OnSuccess`
            (goto _label))
          (:`OnFail`
            (goto _label_2))))
      (:`2`
        (`|AIMoveTo` self (`SceneComponent.K2_GetComponentLocation` (`/Game/FirstPerson/Sanctuary/BP_Sanctum.AttackPoint3` _sanctuaryref)) null
          (:`OnSuccess`
            (goto _label))
          (:`OnFail`
            (goto _label_2))))
      (:`3`
        (`|AIMoveTo` self (`SceneComponent.K2_GetComponentLocation` (`/Game/FirstPerson/Sanctuary/BP_Sanctum.AttackPoint4` _sanctuaryref)) null
          (:`OnSuccess`
            (goto _label))
          (:`OnFail`
            (goto _label_2)))))))

(event `Chase Player`
  (bind _returnvalue (`GameplayStatics.GetPlayerCharacter` 0))
  (bind (_returnvalue_roll _returnvalue_pitch) (`KismetMathLibrary.BreakRotator` (`self.K2_GetActorRotation`)))
  (bind (_returnvalue_roll_2 _returnvalue_pitch_2 _returnvalue_yaw) (`KismetMathLibrary.BreakRotator` (`KismetMathLibrary.FindLookAtRotation` (`self.K2_GetActorLocation`) (`self.K2_GetActorLocation` _returnvalue))))
  (if (not (`self.Dead`))
    (`|AIMoveTo` self (0.0 0.0 0.0) _returnvalue
      (:`OnSuccess`
        (if (not (`self.Dead`))
          (`self.K2_SetActorRotation` (`KismetMathLibrary.MakeRotator` _returnvalue_roll _returnvalue_pitch _returnvalue_yaw))
          (`self.Attack`)
          (set `self.ChasingPlayer` false)))
      (:`OnFail`
        (`KismetSystemLibrary.Delay` 0.2)
        (if (`self.ChasingPlayer`)
          (`self.Chase Player`)
          (else
            (`self.MoveToSanctuary`)))))))

(event `self.ReceiveBeginPlay`
  (bind _returnvalue (`GameplayStatics.GetActorOfClass` "/Game/FirstPerson/Sanctuary/BP_Sanctum.BP_Sanctum_C"))
  (`/Engine/EditorBlueprintResources/StandardMacros.IsValid` _returnvalue
    (:`Is Valid`
      (set `self.SanctuaryRef` _returnvalue)
      (`self.MoveToSanctuary`))))

(event `Bodyshot`
  (bind _health (`self.health`))
  (bind _charactermovement (`self.CharacterMovement`))
  (if (`self.Dead`)
    _
    (elif (> _health 0.0)
      (set `self.health` (- _health 25.0))
      (if (<= _health 0.0)
        (set `self.Dead` true)
        (`GameplayStatics.PlaySound2D` "/Game/Sound/SoundCues/RobotDeath.RobotDeath" 1.0 1.0 0.0 null null)
        (set `CharacterMovementComponent.MaxWalkSpeed` 0.0 (`self.CharacterMovement`))
        (`KismetSystemLibrary.Delay` 3.0)
        (`self.K2_DestroyActor`)
        (else
          (`GameplayStatics.PlaySound2D` "/Game/Sound/SoundCues/BulletHit.BulletHit" 1.0 1.0 0.0 null null)
          (`SkeletalMeshComponent.PlayAnimation` (`self.Mesh`) "/Game/Enemy/Animations/Stomach_Hit.Stomach_Hit" false)
          (set `CharacterMovementComponent.MaxWalkSpeed` 0.0 _charactermovement)
          (`KismetSystemLibrary.Delay` 0.4)
          (`SkeletalMeshComponent.SetAnimationMode` (`self.Mesh`) "AnimationBlueprint")
          (set `CharacterMovementComponent.MaxWalkSpeed` 450.0 _charactermovement))))))

(event `self.CapsuleComponent.OnComponentHit`
  (params (HitComponent :type "PrimitiveComponent Object Reference") (OtherActor :type "Actor Object Reference") (OtherComp :type "PrimitiveComponent Object Reference") (NormalImpulse :type "Vector Structure") (Hit :type "HitResult Structure (by ref)")))

(event `Headshot`
  (bind _health (`self.health`))
  (if (`self.Dead`)
    _
    (elif (> _health 0.0)
      (set `self.health` (- _health 100.0))
      (if (<= _health 0.0)
        (set `self.Dead` true)
        (`GameplayStatics.PlaySound2D` "/Game/Sound/SoundCues/RobotDeath.RobotDeath" 1.0 1.0 0.0 null null)
        (set `CharacterMovementComponent.MaxWalkSpeed` 0.0 (`self.CharacterMovement`))
        (`KismetSystemLibrary.Delay` 3.0)
        (`self.K2_DestroyActor`)))))

(event `self.Head Sphere Collision .OnComponentHit`
  (params (HitComponent :type "PrimitiveComponent Object Reference") (OtherActor :type "Actor Object Reference") (OtherComp :type "PrimitiveComponent Object Reference") (NormalImpulse :type "Vector Structure") (Hit :type "HitResult Structure (by ref)")))

(event `self.PawnSensing.OnSeePawn`
  (params (Pawn :type "Pawn Object Reference"))
  (cast `/Game/FirstPerson/Blueprints/BP_FirstPersonCharacter` Pawn)
  (set `self.ChasingPlayer` true)
  (`self.Chase Player`))

(event `self.ReceiveTick`
  (params (DeltaSeconds :type "Float (single-precision)"))
  (if (and (`self.Dead`) (> (`KismetMathLibrary.VSize` (`self.GetVelocity`)) 0.0))
    (set `CharacterMovementComponent.MaxWalkSpeed` 0.0 (`self.CharacterMovement`))
    (`KismetSystemLibrary.PrintString` "HOTFIX")))

(fn `UserConstructionScript`)